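; Game mode for a Breakout game that tracks remaining balls, block counts and the win or lose state.
; An Action call spawns a ball at a TargetPoint and updates the HUD's ball count, or reloads the level after game over.
; Block add and break counters trigger the clear widget and pause when none remain.
; A miss with no balls left shows the game-over widget.
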(event EventBeginPlay
  (Variables|Default|SetLeftBallNum 3)
  (Variables|Default|SetIsBallSpawned false)
  (Variables|Default|SetIsGameOver false)
  (Variables|Default|SetGameEnded false)
  (CallFunction|ViewGameInformation))

(event EventTick
  (params (DeltaSeconds :type Float%20%28single-precision%29)))

(fn ConstructionScript)

(fn ViewGameOverWidget
  (bind _returnvalue (UserInterface|CreateWidget "/Game/Breakout/GameOverWidget.GameOverWidget_C"))
  (UserInterface|Viewport|AddtoViewport _returnvalue 0))

(fn MissCount
  (Variables|Default|SetIsBallSpawned false)
  (if (and (not (Variables|Default|GetIsCleared)) (not (Variables|Default|GetGameEnded)))
    (Math|Integer|CompareInt (Variables|Default|GetLeftBallNum) 0
      (:==
        (Variables|Default|SetIsGameOver true)
        (Variables|Default|SetGameEnded true)
        (CallFunction|ViewGameOverWidget)))))

(fn ViewClearWidget
  (bind _returnvalue (UserInterface|CreateWidget "/Game/Breakout/ClearWidget.ClearWidget_C"))
  (UserInterface|Viewport|AddtoViewport _returnvalue 0))

(fn AddBlockNum
  (Variables|Default|SetBlockNum (+ (Variables|Default|GetBlockNum) 1))
  (Development|PrintString "AddBlockNum："))

(fn AddBrokenBlockNum
  (Variables|Default|SetBrokenBlockNum (+ (Variables|Default|GetBrokenBlockNum) 1))
  (Development|PrintString "BrokenBlockNum：")
  (bind _leftblocknum (CallFunction|GetLeftBlockNum))
  (if (and (== _leftblocknum 0) (not (Variables|Default|GetGameEnded)))
    (Variables|Default|SetIsCleared true)
    (Variables|Default|SetGameEnded true)
    (CallFunction|ViewClearWidget)
    (Game|SetGamePaused true)))

(fn GetLeftBlockNum
  (bind _blocknum (Variables|Default|GetBlockNum))
  (bind _brokenblocknum (Variables|Default|GetBrokenBlockNum))
  (bind _returnvalue (- _blocknum _brokenblocknum))
  (Development|PrintString (Utilities|String|Append "LeftBlockNum：" (Utilities|String|ToString(Integer) _returnvalue)))
  (return _returnvalue))

(fn ViewGameInformation
  (bind _returnvalue (UserInterface|CreateWidget "/Game/Breakout/GameInformation.GameInformation_C"))
  (UserInterface|Viewport|AddtoViewport _returnvalue 0)
  (bind _output_get (Variables|Default|SetGameInformationWidget _returnvalue))
  (Default|UpdateLeftBallNum _output_get (Variables|Default|GetLeftBallNum)))

(fn UpdateLeftBallDisplay
  (Default|UpdateLeftBallNum (Variables|Default|GetGameInformationWidget) (Variables|Default|GetLeftBallNum)))

(fn Action
  (if (Variables|Default|GetIsGameOver)
    (CallFunction|LevelReset)
    (elif (not (Variables|Default|GetIsCleared))
      (if (not (Variables|Default|GetIsBallSpawned))
        (CallFunction|SpawnBall)))))

(fn LevelReset
  (Game|OpenLevel(byName) "L_InGame"))

(fn SpawnBall
  (if (not (Variables|Default|GetIsBallSpawned))
    (bind _returnvalue (Actor|GetActorOfClass "/Script/Engine.TargetPoint"))
    (Game|SpawnActorfromClass "/Game/Breakout/BP_Ball.BP_Ball_C" (Transformation|GetActorTransform _returnvalue) "AlwaysSpawn" "MultiplyWithRoot" 0 0)
    (Variables|Default|SetIsBallSpawned true)
    (bind _result (Math|Integer|DecrementInt (Variables|Default|GetLeftBallNum))
      (:%20%20
        (Variables|Default|SetLeftBallNum _result)
        (CallFunction|UpdateLeftBallDisplay)))))